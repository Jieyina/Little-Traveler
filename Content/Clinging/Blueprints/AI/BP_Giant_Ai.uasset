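; BP_Giant_Ai is a climbable giant boss that fights characters and registers itself as the player's boss while the player is in range.
; On begin play it hands itself to BPAIHandler and registers its body-part cling objects with BPFactionComponent.
; Damage goes through the faction component, which updates the giant's health values.
; Detection overlaps add and remove AI targets, and an interface event forwards changes in clinging characters to the handler.
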(event `self.ReceiveBeginPlay`
  ;[1 0.8064 0.3944] BeginPlay
  ;;[1 1 1] Sets the ClingObjects that can attack in the array
  (set `/Game/Clinging/Blueprints/AI/BP_AI_Handler.Character` self (`self.BP_AI_Handler`))
  ;;[1 1 1] Puts all Clingobjects In an array
  (`/Game/Clinging/Blueprints/BP_FactionComponent.SetupClingObjects` (`self.BP_FactionComponent`) true (`|MakeArray` (`self.Cling_Spine01`) (`self.Cling_ArmL`) (`self.Cling_UpperArmL`) (`self.Cling_ArmR`) (`self.Cling_UpperArmR`) (`self.Cling_Head`) (`self.Cling_Spine03`) (`self.Cling_ThighL`) (`self.Cling_ThighR`) (`self.Cling_CalfL`) (`self.Cling_CalfR`))))

(event `self.ReceiveAnyDamage`
  (params (Damage :type "Float (single-precision)") (DamageType :type "DamageType Object Reference") (InstigatedBy :type "Controller Object Reference") (DamageCauser :type "Actor Object Reference"))
  (bind _bp_factioncomponent (`self.BP_FactionComponent`))
  ;[0.9479 0.7873 0.4295] Damaged
  (`/Game/Clinging/Blueprints/BP_FactionComponent.ModifyHealth` _bp_factioncomponent Damage self)
  (`/Engine/EditorBlueprintResources/StandardMacros.IsValid` _bp_factioncomponent
    (:`Is Valid`
      (set `self.Health` (`/Game/Clinging/Blueprints/BP_FactionComponent.Health` _bp_factioncomponent)))
    (:`Is Not Valid`
      _))
  (`/Engine/EditorBlueprintResources/StandardMacros.IsValid` _bp_factioncomponent
    (:`Is Valid`
      (set `self.MaxHealth` (`/Game/Clinging/Blueprints/BP_FactionComponent.MaxHealth` _bp_factioncomponent)))))

(event `/Game/Clinging/Blueprints/Interfaces/BI_ClingPawn.ModifyClingCharacters`
  (params (`Add?` :type Boolean) (Actor :type "Actor Object Reference"))
  ;[1 0.8064 0.3944] Interface events
  (`/Game/Clinging/Blueprints/AI/BP_AI_Handler.ModifyClingTargets` (`self.BP_AI_Handler`) `Add?` Actor))

(event `self.Detection.OnComponentBeginOverlap`
  (params (OverlappedComponent :type "PrimitiveComponent Object Reference") (OtherActor :type "Actor Object Reference") (OtherComp :type "PrimitiveComponent Object Reference") (OtherBodyIndex :type Integer) (bFromSweep :type Boolean) (SweepResult :type "HitResult Structure (by ref)"))
  ;[1 0.8064 0.3944] Detect Enemies
  (bind _asbp_climbing_character (cast `/Game/Clinging/Blueprints/BP_ClimbingCharacter` OtherActor)
    (:`then`
      (if (== _asbp_climbing_character (`GameplayStatics.GetPlayerCharacter` 0))
        (set `/Game/Clinging/Blueprints/BP_ClimbingCharacter.Boss` self _asbp_climbing_character)))
    (:`CastFailed`
      _))
  (`/Game/Clinging/Blueprints/AI/BP_AI_Handler.AddTarget` (`self.BP_AI_Handler`) OtherActor))

(event `self.Detection.OnComponentEndOverlap`
  (params (OverlappedComponent :type "PrimitiveComponent Object Reference") (OtherActor :type "Actor Object Reference") (OtherComp :type "PrimitiveComponent Object Reference") (OtherBodyIndex :type Integer))
  ;[1 0.8064 0.3944] Detect Enemies
  (bind _asbp_climbing_character (cast `/Game/Clinging/Blueprints/BP_ClimbingCharacter` OtherActor)
    (:`then`
      (if (== _asbp_climbing_character (`GameplayStatics.GetPlayerCharacter` 0))
        (set `/Game/Clinging/Blueprints/BP_ClimbingCharacter.Boss` null _asbp_climbing_character)))
    (:`CastFailed`
      _))
  (`/Game/Clinging/Blueprints/AI/BP_AI_Handler.RemoveTarget` (`self.BP_AI_Handler`) OtherActor))

(fn `UserConstructionScript`)