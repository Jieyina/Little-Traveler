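; AI handler that drives a Character through roam, patrol, chase and attack against non-allied faction targets, with support for clinging climbers.
; A looping timer runs the state logic; despite its name, GetRandomTarget picks the nearest target.
; Attacks randomly play a flail montage, which flails a climbing target, or distance-based melee/ranged montages.
; Helpers handle socket sphere-trace damage with hit pauses, montage turns via BP_LerpTimer, and target limb lookup.
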(event `self.ReceiveBeginPlay`
  (bind _returnvalue (`Actor.GetComponentByClass` (`self.Character`) "/Game/Clinging/Blueprints/Components/BP_ClingComponent.BP_ClingComponent_C"))
  (set `self.State` (`self.DefaultState`))
  (bind _returnvalue_2 (`KismetSystemLibrary.K2_SetTimer` null "Update" 0.1 true))
  (set `self.UpdateTimer` _returnvalue_2)
  (if (`self.CanClimb?`)
    (`/Engine/EditorBlueprintResources/StandardMacros.IsValid` _returnvalue
      (:`Is Valid`
        (set `self.ClingComp` _returnvalue))
      (:`Is Not Valid`
        (set `self.CanClimb?` false)))))

(event `CheckTargetIsClimbing`
  ;[0.9479 0.7873 0.4295] Comment
  (if (`KismetArrayLibrary.Array_Contains` (`self.ClingTargets`) (`self.CurTarget`))
    (set `self.TargetIsClimbing` true)
    (else
      (set `self.TargetIsClimbing` false))))

(event `Update`
  ;[0.9479 0.7873 0.4295] Comment
  (if (`self.Dummy?`)
    _
    (elif (`self.Dead?`)
      _
      (elif (`self.Ignore`)
        _
        (elif (`self.HasTarget`)
          (`self.State_Chase`)
          (else
            (switch `/Game/Clinging/Blueprints/AI/States` (`self.State`)
              (:`NewEnumerator1`
                (`self.State_Roam`))
              (:`NewEnumerator5`
                (`self.State_Patrol`)))))))))

(event `ModifyClingTargets`
  (params (`Add?` :type Boolean) (Actor :type "Actor Object Reference"))
  (bind _clingtargets (`self.ClingTargets`))
  (bind _clingtargets_2 (`self.ClingTargets`))
  ;[0.9479 0.7873 0.4295] Comment
  (if `Add?`
    (if (not (`KismetArrayLibrary.Array_Contains` _clingtargets Actor))
      (`KismetArrayLibrary.Array_AddUnique` _clingtargets Actor))
    (elif (`KismetArrayLibrary.Array_Contains` _clingtargets_2 Actor)
      (`KismetArrayLibrary.Array_RemoveItem` _clingtargets_2 Actor))))

(event `Attack`
  (bind _curtarget (`self.CurTarget`))
  (bind _curtarget_2 (`self.CurTarget`))
  (bind _returnvalue (<= (`self.Distance`) (`self.MeleeDistance`)))
  (bind _mesh (`Character.Mesh` (`self.Character`)))
  ;[0.9479 0.7873 0.4295] This randomizes attacks between all of them or just the Roar that flails all cling targets based on if the current target is climbing or not
  (set `self.State` "NewEnumerator4")
  (if (`self.Turning`)
    _
    (elif (`self.TurnToActor?` _curtarget)
      (`/Engine/EditorBlueprintResources/StandardMacros.DoOnce` false :!label _label
        (:`Completed`
          (`self.TurnActor` _curtarget)))
      (elif (not (`self.Attacking`))
        (set `self.Attacking` true)
        (if (< (`KismetMathLibrary.RandomIntegerInRange` 0 100) (`self.FlailChance`))
          (`|PlayMontage` _mesh (`self.FlailMontage`) 1.0 0.0 "None"
            (:`then`
              (if (`self.TargetIsClimbing`)
                (message `/Game/Clinging/Blueprints/Interfaces/BI_ClingPawn.FlailActor` _curtarget_2 true)))
            (:`OnCompleted`
              (message `/Game/Clinging/Blueprints/Interfaces/BI_ClingPawn.FlailActor` _curtarget_2 false :!label _label_2)
              (`|ExecutionSequence`
                (:`then_0`
                  (`self.Reset`))
                (:`then_1`
                  (goto _label :!via `Reset`))))
            (:`OnInterrupted`
              (goto _label_2)))
          (else
            (`|PlayMontage` _mesh (select `bool` _returnvalue :`false` (`self.RangedMontage`) :`true` (`self.MeleeMontage`)) 1.0 0.0 (`KismetStringLibrary.Conv_StringToName` (`KismetStringLibrary.Conv_IntToString` (`KismetMathLibrary.RandomIntegerInRange` 1 (select `bool` _returnvalue :`false` (`self.RangedMax`) :`true` (`self.MeleeMax`)))))
              (:`OnCompleted`
                _)
              (:`OnInterrupted`
                _))
            (`KismetArrayLibrary.Array_Clear` (`self.HitTargets`))
            (`|ExecutionSequence`
              (:`then_0`
                (`self.Reset`))
              (:`then_1`
                (goto _label :!via `Reset`)))))))))

(event `HitPause`
  (params (Duration :type "Float (double-precision)"))
  (bind _mesh (`Character.Mesh` (`self.Character`)))
  ;[0.9479 0.7873 0.4295] Comment
  (set `SkeletalMeshComponent.bPauseAnims` true _mesh)
  (`KismetSystemLibrary.Delay` Duration)
  (set `SkeletalMeshComponent.bPauseAnims` false _mesh))

(event `AddTarget`
  (params (Actor :type "Actor Object Reference"))
  (bind _returnvalue (`Actor.GetComponentByClass` Actor "/Game/Clinging/Blueprints/BP_FactionComponent.BP_FactionComponent_C"))
  (bind _potentialtargets (`self.PotentialTargets`))
  (bind _returnvalue_2 (`Actor.GetComponentByClass` (`self.Character`) "/Game/Clinging/Blueprints/BP_FactionComponent.BP_FactionComponent_C"))
  ;[0.9479 0.7873 0.4295] Comment
  (`/Engine/EditorBlueprintResources/StandardMacros.IsValid` _returnvalue
    (:`Is Valid`
      (`/Engine/EditorBlueprintResources/StandardMacros.IsValid` _returnvalue_2
        (:`Is Valid`
          (if (`KismetArrayLibrary.Array_Contains` (`/Game/Clinging/Blueprints/BP_FactionComponent.Allies` _returnvalue_2) (`/Game/Clinging/Blueprints/BP_FactionComponent.Faction` _returnvalue))
            _
            (elif (not (`KismetArrayLibrary.Array_Contains` _potentialtargets Actor))
              (`KismetArrayLibrary.Array_Add` _potentialtargets Actor)
              (set `self.HasTarget` true)
              (set `self.CurTarget` Actor)
              (`self.GetRandomTarget`))))))))

(event `State_Chase`
  ;[1 0.8064 0.3944] Chase State
  (if (not (`self.Turning`))
    (`self.Chase`)))

(event `AttackTraces`
  (params (PrimaryStart :type Name) (PrimaryEnd :type Name) (Radius :type "Float (double-precision)"))
  (bind _character (`self.Character`))
  (bind _mesh (`Character.Mesh` _character))
  ;[0.9479 0.7873 0.4295] Comment
  (bind (_outhits _returnvalue) (`KismetSystemLibrary.SphereTraceMulti` :`Start` (`SceneComponent.GetSocketLocation` _mesh PrimaryStart) :`End` (`SceneComponent.GetSocketLocation` _mesh PrimaryEnd) :`Radius` (* (.x (.scale (`Actor.GetTransform` _character))) Radius) :`TraceChannel` "TraceTypeQuery4" :`DrawDebugType` "ForOneFrame"))
  (if _returnvalue
    (for _array_element _outhits
      (bind (_bblockinghit _binitialoverlap _time _distance _location _impactpoint _normal _impactnormal _physmat _hitactor _hitcomponent) (`GameplayStatics.BreakHitResult` _array_element))
      (if (not (`KismetArrayLibrary.Array_Contains` (`self.HitTargets`) _hitactor))
        (`KismetArrayLibrary.Array_AddUnique` (`self.HitTargets`) _hitactor)
        (if (not (`KismetArrayLibrary.Array_Contains` (`SceneComponent.GetChildrenComponents` (`Character.Mesh` (`self.Character`)) true) _hitcomponent))
          (bind _asbp_base_cling_object (cast `/Game/Clinging/Blueprints/Components/BP_BaseClingObject` _hitactor)
            (:`then`
              (if (not (`KismetArrayLibrary.Array_Contains` (`self.AllLimbObjects`) _asbp_base_cling_object))
                (`GameplayStatics.ApplyDamage` _hitactor 10.0 null (`self.Character`) :!label _label_3)
                (`self.HitPause` 0.1)))
            (:`CastFailed`
              (goto _label_3))))))))

(event `State_Patrol`
  (bind _output (`|GetArrayItem` (`self.PatrolPoints`) (`self.PatrolPointIndex`)))
  ;[1 0.8064 0.3944] Patrol State
  (set `self.State` "NewEnumerator5")
  (if (`self.Turning`)
    _
    (elif (not (`self.Patrolling`))
      (set `self.Patrolling` true)
      (if (`self.TurnToActor?` _output)
        (`/Engine/EditorBlueprintResources/StandardMacros.DoOnce` false :!label _label_4
          (:`Completed`
            (`self.TurnActor` _output)))
        (else
          (`|AIMoveTo` (`self.Character`) (0.0 0.0 0.0) _output
            (:`OnSuccess`
              (`/Engine/EditorBlueprintResources/StandardMacros.IncrementInt` (`self.PatrolPointIndex`)
                (:`  `
                  _)))
            (:`OnFail`
              _))
          (if (== (`self.PatrolPointIndex`) (`KismetArrayLibrary.Array_Length` (`self.PatrolPoints`)))
            (set `self.PatrolPointIndex` 0))
          (`KismetSystemLibrary.Delay` 3.0)
          (set `self.Patrolling` false)
          (goto _label_4 :!via `Reset`))))))

(event `Chase`
  (bind _character (`self.Character`))
  (bind _curtarget (`self.CurTarget`))
  (bind _returnvalue (`KismetMathLibrary.VSize` (- (`Actor.K2_GetActorLocation` _character) (`Actor.K2_GetActorLocation` _curtarget))))
  ;[0.9479 0.7873 0.4295] Comment
  (if (`self.HasTarget`)
    (`/Engine/EditorBlueprintResources/StandardMacros.IsValid` (`self.CurTarget`)
      (:`Is Valid`
        (`|ExecutionSequence`
          (:`then_0`
            (`self.CheckTargetIsClimbing`)
            (if (not (`self.TargetIsClimbing`))
              (`|AIMoveTo` _character (0.0 0.0 0.0) _curtarget
                (:`then`
                  (set `self.Distance` _returnvalue)
                  (if (< _returnvalue (`self.CombatDistance`))
                    (set `self.InRange` true)
                    (if (< (`KismetMathLibrary.RandomIntegerInRange` 0 100) (`self.AttackChance`))
                      (`self.Attack`))
                    (else
                      (set `self.InRange` false)))))))
          (:`then_1`
            (goto _label_5 :!via `Reset`))))
      (:`Is Not Valid`
        (`/Engine/EditorBlueprintResources/StandardMacros.DoOnce` false :!label _label_5
          (:`Completed`
            (`self.GetRandomTarget`)))))
    (else
      (`self.GetRandomTarget`))))

(event `State_Roam`
  ;[1 0.8064 0.3944] Roam State
  (set `self.State` "NewEnumerator1")
  (if (`self.Turning`)
    _
    (elif (not (`self.isRoaming`))
      (set `self.isRoaming` true)
      (bind _output_get (set `self.RoamLocation` (`NavigationSystemV1.K2_GetRandomLocationInNavigableRadius` (`Actor.K2_GetActorLocation` (`self.Character`)) 1000.0 null null)))
      (`|AIMoveTo` (`self.Character`) _output_get null 50.0
        (:`OnSuccess`
          (`KismetSystemLibrary.Delay` 3.0)
          (set `self.isRoaming` false))))))

(event `TurnLoc`
  (params (Target :type "Vector Structure (by ref)"))
  (bind (_rotation _right) (`self.GetLookAtRotationLoc` Target))
  (bind _character (`self.Character`))
  (bind _returnvalue (`KismetMathLibrary.MakeTransform` (0.0 0.0 0.0) (`Actor.K2_GetActorRotation` _character)))
  ;[0.9479 0.7873 0.4295] Turn
  (`self.LerpTimer`
    (:`then`)
    (:`else`
      (if (not (`self.Turning`))
        (set `self.Turning` true)
        (if (`self.TurnToLocation?` Target)
          (`Character.PlayAnimMontage` (`self.Character`) (`self.TurnMontage`) 1.0 (select `bool` _right :`false` "Left" :`true` "Right" :!type "Name"))
          (bind _returnvalue_2 (`|SpawnActorFromClass` "/Game/Clinging/Blueprints/Components/BP_LerpTimer.BP_LerpTimer_C" _returnvalue "AlwaysSpawn" "OverrideRootScale" null _character null false true 1.0 _returnvalue (`KismetMathLibrary.MakeTransform` (0.0 0.0 0.0) _rotation) null))
          (set `self.LerpTimer` _returnvalue_2)
          (`KismetSystemLibrary.Delay` 1.0))
        (set `self.Turning` false)
        (set `self.LerpTimer` null)))))

(event `Reset`
  (bind _hastarget (`self.HasTarget`))
  ;[1 0.8064 0.3944] Reset variables
  (set `self.Attacking` false)
  (set `self.Turning` false)
  (set `self.Trace` false)
  (set `self.State` (select `bool` _hastarget :`false` (`self.DefaultState`) :`true` "NewEnumerator4"))
  (if _hastarget
    (`self.GetRandomTarget`)))

(event `RemoveTarget`
  (params (Actor :type "Actor Object Reference"))
  (bind _potentialtargets (`self.PotentialTargets`))
  ;[0.9479 0.7873 0.4295] Comment
  (if (`KismetArrayLibrary.Array_Contains` _potentialtargets Actor)
    (`KismetArrayLibrary.Array_RemoveItem` _potentialtargets Actor)
    (`self.GetRandomTarget`)))

(event `TurnActor`
  (params (Target :type "Actor Object Reference"))
  (bind (_rotation _right) (`self.GetLookAtRotationActor` Target))
  (bind _character (`self.Character`))
  (bind _returnvalue (`KismetMathLibrary.MakeTransform` (0.0 0.0 0.0) (`Actor.K2_GetActorRotation` _character)))
  ;[0.9479 0.7873 0.4295] Turn
  (`self.LerpTimer`
    (:`then`)
    (:`else`
      (if (not (`self.Turning`))
        (set `self.Turning` true)
        (if (`self.TurnToActor?` Target)
          (`Character.PlayAnimMontage` (`self.Character`) (`self.TurnMontage`) 1.0 (select `bool` _right :`false` "Left" :`true` "Right" :!type "Name"))
          (bind _returnvalue_2 (`|SpawnActorFromClass` "/Game/Clinging/Blueprints/Components/BP_LerpTimer.BP_LerpTimer_C" _returnvalue "AlwaysSpawn" "OverrideRootScale" null _character null false true 1.0 _returnvalue (`KismetMathLibrary.MakeTransform` (0.0 0.0 0.0) _rotation) null))
          (set `self.LerpTimer` _returnvalue_2)
          (`KismetSystemLibrary.Delay` 1.0))
        (set `self.Turning` false)
        (set `self.LerpTimer` null)))))

(fn `GetClosestObjectOnTarget`
  (returns (ClosestObject :type "/Game/Clinging/Blueprints/Components/BP_BaseClingObject Object Reference"))
  (locals (CycleDIs :type "Float (double-precision)" :default 100000.0) (LocalObject :type "/Game/Clinging/Blueprints/Components/BP_BaseClingObject Object Reference"))
  (bind _returnvalue (`Actor.GetComponentByClass` (`self.CurTarget`) "/Game/Clinging/Blueprints/BP_FactionComponent.BP_FactionComponent_C"))
  (`/Engine/EditorBlueprintResources/StandardMacros.IsValid` _returnvalue
    (:`Is Valid`
      (set `local.CycleDIs` 100000.0)
      (for _array_element (`/Game/Clinging/Blueprints/BP_FactionComponent.AllLimbObjects` _returnvalue)
        (bind _returnvalue_2 (`Actor.GetDistanceTo` (`self.Character`) _array_element))
        (if (<= _returnvalue_2 (`local.CycleDIs`))
          (set `local.CycleDIs` _returnvalue_2)
          (set `local.LocalObject` _array_element))))
    (:`Is Not Valid`
      (set `local.LocalObject` null)))
  (return (`local.LocalObject`)))

(fn `GetIsClinging`
  (returns (`Clinging?` :type Boolean))
  (bind _clingcomp (`self.ClingComp`))
  (`/Engine/EditorBlueprintResources/StandardMacros.IsValid` _clingcomp
    (:`Is Valid`
      (return (`/Game/Clinging/Blueprints/Components/BP_ClingComponent.isClinging` _clingcomp)))
    (:`Is Not Valid`
      (return false))))

(fn `GetLookAtRotationActor`
  (params (Target :type "Actor Object Reference"))
  (returns (Rotation :type "Rotator Structure") (Right :type Boolean))
  (bind _character (`self.Character`))
  (bind (_returnvalue_roll _returnvalue_pitch) (`KismetMathLibrary.BreakRotator` (`Actor.K2_GetActorRotation` _character)))
  (bind _returnvalue (`KismetMathLibrary.FindLookAtRotation` (`Actor.K2_GetActorLocation` _character) (`Actor.K2_GetActorLocation` Target)))
  (bind (_returnvalue_roll_2 _returnvalue_pitch_2 _returnvalue_yaw) (`KismetMathLibrary.BreakRotator` (`KismetMathLibrary.NormalizedDeltaRotator` _returnvalue (`Actor.K2_GetActorRotation` _character))))
  (return (`KismetMathLibrary.MakeRotator` _returnvalue_roll _returnvalue_pitch (.yaw _returnvalue)) (> _returnvalue_yaw 0.0)))

(fn `GetLookAtRotationLoc`
  (params (Target :type "Vector Structure (by ref)"))
  (returns (Rotation :type "Rotator Structure") (Right :type Boolean))
  (bind _character (`self.Character`))
  (bind (_returnvalue_roll _returnvalue_pitch) (`KismetMathLibrary.BreakRotator` (`Actor.K2_GetActorRotation` _character)))
  (bind _returnvalue (`KismetMathLibrary.FindLookAtRotation` (`Actor.K2_GetActorLocation` _character) Target))
  (bind (_returnvalue_roll_2 _returnvalue_pitch_2 _returnvalue_yaw) (`KismetMathLibrary.BreakRotator` (`KismetMathLibrary.NormalizedDeltaRotator` _returnvalue (`Actor.K2_GetActorRotation` _character))))
  (return (`KismetMathLibrary.MakeRotator` _returnvalue_roll _returnvalue_pitch (.yaw _returnvalue)) (> _returnvalue_yaw 0.0)))

(fn `GetObjectOnTarget`
  (params (Type :type "/Game/Clinging/Blueprints/Components/E_ClingType Enum" :default "NewEnumerator0") (`All?` :type Boolean))
  (returns (ClosestObject :type "/Game/Clinging/Blueprints/Components/BP_BaseClingObject Object Reference"))
  (locals (CycleDIs :type "Float (double-precision)" :default 100000.0) (LocalObject :type "/Game/Clinging/Blueprints/Components/BP_BaseClingObject Object Reference"))
  (bind _returnvalue (`Actor.GetComponentByClass` (`self.CurTarget`) "/Game/Clinging/Blueprints/BP_FactionComponent.BP_FactionComponent_C"))
  (bind _returnvalue_2 (select `bool` `All?` :`false` (select `/Game/Clinging/Blueprints/Components/E_ClingType` Type :`NewEnumerator0` (`/Game/Clinging/Blueprints/BP_FactionComponent.AllNeutrals` _returnvalue) :`NewEnumerator1` (`/Game/Clinging/Blueprints/BP_FactionComponent.AllArmored` _returnvalue) :`NewEnumerator2` (`/Game/Clinging/Blueprints/BP_FactionComponent.AllWeaknesses` _returnvalue)) :`true` (`/Game/Clinging/Blueprints/BP_FactionComponent.AllLimbObjects` _returnvalue)))
  (`/Engine/EditorBlueprintResources/StandardMacros.IsValid` _returnvalue
    (:`Is Valid`
      (bind _output_get (set `local.LocalObject` (`|GetArrayItem` _returnvalue_2 (- (`KismetArrayLibrary.Array_Length` _returnvalue_2) 1))))
      (return _output_get))
    (:`Is Not Valid`
      (return null))))

(fn `GetRandomTarget`
  (locals (MaxDistance :type "Float (double-precision)" :default 0.0))
  (if (> (`KismetArrayLibrary.Array_Length` (`self.PotentialTargets`)) 0)
    (set `local.MaxDistance` 100000.0)
    (for _array_element (`self.PotentialTargets`)
      (bind _returnvalue (`Actor.GetDistanceTo` (`self.Character`) _array_element))
      (if (< _returnvalue (`local.MaxDistance`))
        (set `local.MaxDistance` _returnvalue)
        (set `self.CurTarget` _array_element)
        (set `self.HasTarget` true)))
    (set `self.State` "NewEnumerator2")
    (else
      (set `self.HasTarget` false)
      (set `self.State` (`self.DefaultState`)))))

(fn `TurnToActor?`
  (params (Target :type "Actor Object Reference"))
  (returns (Turn :type Boolean))
  (bind _character (`self.Character`))
  (bind (_returnvalue_roll _returnvalue_pitch _returnvalue_yaw) (`KismetMathLibrary.BreakRotator` (`KismetMathLibrary.NormalizedDeltaRotator` (`KismetMathLibrary.FindLookAtRotation` (`Actor.K2_GetActorLocation` _character) (`Actor.K2_GetActorLocation` Target)) (`Actor.K2_GetActorRotation` _character))))
  (return (> (`KismetMathLibrary.Abs` _returnvalue_yaw) 50.0)))

(fn `TurnToLocation?`
  (params (Target :type "Vector Structure (by ref)"))
  (returns (Turn :type Boolean))
  (bind _character (`self.Character`))
  (bind (_returnvalue_roll _returnvalue_pitch _returnvalue_yaw) (`KismetMathLibrary.BreakRotator` (`KismetMathLibrary.NormalizedDeltaRotator` (`KismetMathLibrary.FindLookAtRotation` (`Actor.K2_GetActorLocation` _character) Target) (`Actor.K2_GetActorRotation` _character))))
  (return (> (`KismetMathLibrary.Abs` _returnvalue_yaw) 50.0)))