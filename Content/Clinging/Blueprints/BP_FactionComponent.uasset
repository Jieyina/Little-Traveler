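; Faction component for the clinging system that tracks a set of cling objects and a health pool.
; SetupClingObjects casts each supplied child actor to BP_BaseClingObject, adds it uniquely to the limb list and sorts it by type into neutral, armored or weakness arrays.
; ModifyHealth subtracts damage from health and destroys the passed-in target actor when health reaches zero or below.
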(event `SetupClingObjects`
  (params (HasObjects :type Boolean) (Objects :type "Array of ChildActorComponent Object Reference"))
  ;[0.9479 0.7873 0.4295] Comment
  (if HasObjects
    (for _array_element Objects
      (bind _asbp_base_cling_object (cast `/Game/Clinging/Blueprints/Components/BP_BaseClingObject` (`ChildActorComponent.ChildActor` _array_element) :!pure true))
      (`KismetArrayLibrary.Array_AddUnique` (`self.AllLimbObjects`) _asbp_base_cling_object)
      (switch `/Game/Clinging/Blueprints/Components/E_ClingType` (`/Game/Clinging/Blueprints/Components/BP_BaseClingObject.Type` _asbp_base_cling_object)
        (:`NewEnumerator0`
          (`KismetArrayLibrary.Array_Add` (`self.AllNeutrals`) _asbp_base_cling_object))
        (:`NewEnumerator1`
          (`KismetArrayLibrary.Array_Add` (`self.AllArmored`) _asbp_base_cling_object))
        (:`NewEnumerator2`
          (`KismetArrayLibrary.Array_Add` (`self.AllWeaknesses`) _asbp_base_cling_object))))))

(event `ModifyHealth`
  (params (Damage :type "Float (double-precision)") (Target :type "Actor Object Reference"))
  ;[0.9479 0.7873 0.4295] Comment
  (set `self.Health` (- (`self.Health`) Damage))
  (if (<= (`self.Health`) 0.0)
    (`Actor.K2_DestroyActor` Target)))