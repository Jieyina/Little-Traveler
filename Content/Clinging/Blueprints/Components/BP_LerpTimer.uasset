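; Short-lived helper actor that moves and/or rotates a Character from a start to an end transform over a set duration, then destroys itself.
; A Timeline drives curve-eased lerps between two point components.
; When the character is clinging, the points attach to the cling object to follow it.
; While clinging, it also suspends cling ticking, capsule collision and local player input, restoring them on finish with query-only collision.
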(event `self.ReceiveBeginPlay`
  (bind _timer (`self.Timer`))
  (bind _clingobject (`self.ClingObject`))
  (bind _startpoint (`self.StartPoint`))
  (bind _character (`self.Character`))
  (bind _character_2 (`self.Character`))
  (bind _character_3 (`self.Character`))
  (bind _clingobject_2 (`self.ClingObject`))
  (bind _endpoint (`self.EndPoint`))
  (bind (_returnvalue_location _returnvalue_rotation) (`KismetMathLibrary.BreakTransform` (`SceneComponent.K2_GetComponentToWorld` (`self.EndPoint`))))
  (bind (_returnvalue_location_2 _returnvalue_rotation_2) (`KismetMathLibrary.BreakTransform` (`SceneComponent.K2_GetComponentToWorld` (`self.StartPoint`))))
  (bind _returnvalue (`CurveFloat.GetFloatValue` (`self.CurveAlpha`) (`KismetMathLibrary.MapRangeClamped` (`TimelineComponent.GetPlaybackPosition` _timer) 0.0 (`self.Duration`) 0.0 1.0)))
  (`SceneComponent.K2_SetWorldTransform` _startpoint (`self.StartTransform`) false false)
  (`self.CharacterClinging?`
    (:`Clinging`
      (`SceneComponent.K2_AttachToComponent` _startpoint (select `/Game/Clinging/Blueprints/Components/E_ClingObjectType` (`/Game/Clinging/Blueprints/Components/BP_BaseClingObject.ObjectType` _clingobject) :`NewEnumerator0` (`/Game/Clinging/Blueprints/Components/BP_BaseClingObject.Capsule` _clingobject) :`NewEnumerator1` (`/Game/Clinging/Blueprints/Components/BP_BaseClingObject.Box` _clingobject) :`NewEnumerator2` (`/Game/Clinging/Blueprints/Components/BP_BaseClingObject.Mesh` _clingobject) :!type "SceneComponent Object Reference") "None" "KeepWorld" "KeepWorld" "KeepWorld" true))
    (:`Not Clinging`
      _))
  (`SceneComponent.K2_SetWorldTransform` _endpoint (`self.EndTransform`) false false)
  (`self.CharacterClinging?`
    (:`Clinging`
      (`SceneComponent.K2_AttachToComponent` _endpoint (select `/Game/Clinging/Blueprints/Components/E_ClingObjectType` (`/Game/Clinging/Blueprints/Components/BP_BaseClingObject.ObjectType` _clingobject_2) :`NewEnumerator0` (`/Game/Clinging/Blueprints/Components/BP_BaseClingObject.Capsule` _clingobject_2) :`NewEnumerator1` (`/Game/Clinging/Blueprints/Components/BP_BaseClingObject.Box` _clingobject_2) :`NewEnumerator2` (`/Game/Clinging/Blueprints/Components/BP_BaseClingObject.Mesh` _clingobject_2) :!type "SceneComponent Object Reference") "None" "KeepWorld" "KeepWorld" "KeepWorld" true)
      (`self.IgnoreTick` true)
      (`PrimitiveComponent.SetCollisionEnabled` (`Character.CapsuleComponent` _character) "NoCollision")
      (if (== (`self.Character`) (`GameplayStatics.GetPlayerCharacter` 0))
        (`self.DisableInput` _character (`GameplayStatics.GetPlayerController` 0))))
    (:`Not Clinging`
      _))
  (`TimelineComponent.SetTimelineLength` _timer (`self.Duration`))
  (`Timeline|Timer` :!via `PlayFromStart`
    (:`Update`
      (if (`self.Location?`)
        (`self.K2_SetActorLocation` _character_3 (`KismetMathLibrary.VLerp` _returnvalue_location_2 _returnvalue_location _returnvalue) false false))
      (if (`self.Rotation?`)
        (`self.K2_SetActorRotation` _character_3 (`KismetMathLibrary.RLerp` _returnvalue_rotation_2 _returnvalue_rotation _returnvalue true) false)))
    (:`Finished`
      (`self.CharacterClinging?`
        (:`Clinging`
          (`self.IgnoreTick` false)
          (`PrimitiveComponent.SetCollisionEnabled` (`Character.CapsuleComponent` _character_2) "QueryOnly")
          (if (== _character_2 (`GameplayStatics.GetPlayerCharacter` 0))
            (`self.EnableInput` _character_2 (`GameplayStatics.GetPlayerController` 0))))
        (:`Not Clinging`
          _))
      (`self.K2_DestroyActor`))))

(fn `UserConstructionScript`)